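; Base playable character Blueprint that handles a one-handed sword's attachment and its attack, draw and sheathe animations.
; BeginPlay creates the sword as a child actor component on the mesh's sword socket, and a reattach event moves it to the right hand.
; Attack plays the next attack montage and signals completion.
; Sheathing reuses the equip montage at a negative play rate, reattaching the sword on blend out.
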(event `self.ReceiveBeginPlay`
  (bind _returnvalue (`AddComponent|NODE_AddChildActorComponent-3`))
  (bind _output_get (set `self.swordMesh` _returnvalue))
  (`SceneComponent.K2_AttachToComponent` _output_get (`self.Mesh`) "swordAttachment" "KeepRelative" "KeepRelative" "KeepRelative" true))

(event `self.ReceiveActorBeginOverlap`
  (params (OtherActor :type "Actor Object Reference")))

(event `self.onAttack`
  (`|PlayMontage` (`self.Mesh`) (`self.GetNextAttackMontage`)
    (:`OnCompleted`
      (`self.OnAttackFinished`))))

(event `self.onWeaponDrawing`
  (`|PlayMontage` (`self.Mesh`) "/Game/Persona/Animations/Swordset/InPlace/Sword1h_Equip_Montage.Sword1h_Equip_Montage" 0.75
    (:`OnBlendOut`
      (set `self.bWeaponDrawing` false)
      (set `self.bWeaponDrawn` true))))

(event `reattachWeapon`
  (`SceneComponent.K2_AttachToComponent` (`self.swordMesh`) (`self.Mesh`) "hand_rSocket" "KeepRelative" "KeepRelative" "KeepRelative" true))

(event `self.onWeaponHideEvent`
  (`|PlayMontage` (`self.Mesh`) "/Game/Persona/Animations/Swordset/InPlace/Sword1h_Equip_Montage.Sword1h_Equip_Montage" -0.75 1.0
    (:`OnBlendOut`
      (`SceneComponent.K2_AttachToComponent` (`self.swordMesh`) (`self.Mesh`) "swordAttachment" "KeepRelative" "KeepRelative" "KeepRelative" true)
      (`self.onWeaponHideFinished`))))

(fn `UserConstructionScript`)